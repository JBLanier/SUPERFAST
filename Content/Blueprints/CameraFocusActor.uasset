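; Rail camera actor that becomes the player view target and follows the leading Character along a looping course.
; Each tick, a recursive search finds each Character's nearest PlayerSpline time in XZ, keeping the furthest and allowing last-to-first-quarter wraparound.
; That time, eased or snapped on large jumps, samples CameraSpline, and Sphere interpolates to that point.
; The construction script previews a debug time and optionally numbers spline points.
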(event EventBeginPlay
  (Game|Player|SetViewTargetwithBlend (Game|GetPlayerController 0) self 0.0 "VTBlend_Linear" 0.0 false))

(event EventActorBeginOverlap
  (params (OtherActor :type Actor%20Object%20Reference)))

(event EventTick
  (params (DeltaSeconds :type Float%20%28single-precision%29))
  (Variables|Default|SetDeltaTime DeltaSeconds)
  (CallFunction|SetDesiredTime)
  (CallFunction|UpdateDesiredTime)
  (CallFunction|UpdateCamera))

(fn ConstructionScript
  (CallFunction|ScrubCameraTime)
  (CallFunction|SetupDebugNumbers))

(fn IsActorOutOfCameraBounds
  (params (Actor :type Actor%20Object%20Reference))
  (bind _returnvalue (Transformation|GetActorLocation Actor))
  (bind _camera (Variables|Default|GetCamera))
  (bind _camera_2 (Variables|Default|GetCamera))
  (bind _returnvalue_2 (Transformation|GetWorldLocation _camera))
  (bind _orthowidth (Variables|/Script/Engine.CameraComponent|GetOrthoWidth _camera_2))
  (bind _returnvalue_3 (/ _orthowidth 2.0))
  (bind _returnvalue_4 (- _returnvalue _returnvalue_2))
  (bind _output_get (LocalVariables|SetMax%20X%20Distance%20From%20Camera _returnvalue_3))
  (bind _output_get_2 (LocalVariables|SetMax%20Z%20Distance%20From%20Camera (/ _returnvalue_3 (Variables|/Script/Engine.CameraComponent|GetAspectRatio (Variables|Default|GetCamera)))))
  (return (or (> (Math|Float|Absolute(Float) (.x _returnvalue_4)) _output_get) (> (Math|Float|Absolute(Float) (.z _returnvalue_4)) _output_get_2))))

(fn SetTargetPawn
  (params (Pawn :type Pawn%20Object%20Reference))
  (Utilities|IsValid 0
    (:Is%20Valid
      (Variables|Default|SetPawnTarget Pawn))))

(fn DeactivateCamera
  (Variables|Default|SetPawnTarget 0))

(fn ScrubCameraTime
  (Transformation|SetWorldLocation (Variables|Default|GetSphere) (Spline|GetLocationatTime (Variables|Default|GetCameraSpline) (Variables|Debug|GetCameraDebugTime) "World" (Variables|Debug|GetConstant%20Velocity)) false false))

(fn SetupDebugNumbers
  (if (Variables|Debug|GetShowDebugNumbers)
    (Utilities|FlowControl|Sequence
      (:then_0
        (CallFunction|AddSplineNumbers (Variables|Default|GetPlayerSpline)))
      (:then_1
        (CallFunction|AddSplineNumbers (Variables|Default|GetCameraSpline))))))

(fn AddSplineNumbers
  (params (Spline :type Spline%20Component%20Object%20Reference))
  (for _index (range 0 (- (Spline|GetNumberOfSplinePoints Spline) 1))
    (bind _returnvalue (AddComponent|AddTextRenderComponent false (Math|Transform|MakeTransform (+ (.Location (Spline|GetLocationandTangentatSplinePoint Spline _index "Local")) "0, 0,5.000000") "0,90.000000, 0" "20.000000,20.000000,20.000000")))
    (Rendering|Components|TextRender|SetText _returnvalue (Utilities|Text|ToText(Integer) _index))))

(fn UpdateDesiredTime
  (if (>= (Math|Float|Absolute(Float) (- (Variables|Default|GetSplineDesiredTime) (Variables|Default|GetSplineCurrentTime))) (Variables|Default|GetTimeDifferenceThreshold))
    (Variables|Default|SetSplineCurrentTime (Variables|Default|GetSplineDesiredTime))
    (else
      (Variables|Default|SetSplineCurrentTime (+ (* (- (Variables|Default|GetSplineDesiredTime) (Variables|Default|GetSplineCurrentTime)) (Variables|Default|GetDeltaTime) 15.0) (Variables|Default|GetSplineCurrentTime)))))
  (Variables|Default|SetCameraDesiredLocation (Spline|GetLocationatTime (Variables|Default|GetCameraSpline) (Variables|Default|GetSplineCurrentTime) "World" (Variables|Debug|GetConstant%20Velocity))))

(fn RecursiveDistanceCheck
  (params (Iteration :type Integer) (StartTime :type Float%20%28single-precision%29) (EndTime :type Float%20%28single-precision%29) (Pawn :type Pawn%20Object%20Reference))
  (bind _returnvalue (Transformation|GetActorLocation Pawn))
  (bind _playerspline (Variables|Default|GetPlayerSpline))
  (bind _constant_velocity (Variables|Debug|GetConstant%20Velocity))
  (bind _returnvalue_2 (Math|Vector|MakeVector (.x _returnvalue) 0.0 (.z _returnvalue)))
  (LocalVariables|SetNum Iteration)
  (LocalVariables|SetStart StartTime)
  (LocalVariables|SetEnd EndTime)
  (LocalVariables|SetStartDistance (Math|Vector|VectorLength (- (Math|Vector|MakeVector (.x (Spline|GetLocationatTime _playerspline (LocalVariables|GetStart) "World" _constant_velocity)) 0.0 (.z (Spline|GetLocationatTime _playerspline (LocalVariables|GetStart) "World" _constant_velocity))) _returnvalue_2)))
  (LocalVariables|SetEndDistance (Math|Vector|VectorLength (- (Math|Vector|MakeVector (.x (Spline|GetLocationatTime _playerspline (LocalVariables|GetEnd) "World" _constant_velocity)) 0.0 (.z (Spline|GetLocationatTime _playerspline (LocalVariables|GetEnd) "World" _constant_velocity))) _returnvalue_2)))
  (if (< (LocalVariables|GetStartDistance) (LocalVariables|GetEndDistance))
    (if (<= (LocalVariables|GetNum) 0)
      (LocalVariables|SetBest (LocalVariables|GetStart) :!label _label)
      (else
        (LocalVariables|SetNum (- (LocalVariables|GetNum) 1))
        (if (<= (LocalVariables|GetStartDistance) (Variables|Default|GetDistanceThreshold))
          (goto _label)
          (else
            (bind _besttime (CallFunction|RecursiveDistanceCheck (LocalVariables|GetNum) (LocalVariables|GetStart) (Math|Float|Lerp (LocalVariables|GetStart) (LocalVariables|GetEnd) 0.9) Pawn))
            (LocalVariables|SetBest _besttime)))))
    (elif (<= (LocalVariables|GetNum) 0)
      (LocalVariables|SetBest (LocalVariables|GetEnd) :!label _label_2)
      (else
        (LocalVariables|SetNum (- (LocalVariables|GetNum) 1))
        (if (<= (LocalVariables|GetEndDistance) (Variables|Default|GetDistanceThreshold))
          (goto _label_2)
          (else
            (bind _besttime_2 (CallFunction|RecursiveDistanceCheck (LocalVariables|GetNum) (Math|Float|Lerp (LocalVariables|GetStart) (LocalVariables|GetEnd) 0.1) (LocalVariables|GetEnd) Pawn))
            (LocalVariables|SetBest _besttime_2))))))
  (return (LocalVariables|GetBest)))

(fn UpdateCamera
  (Transformation|SetWorldLocation (Variables|Default|GetSphere) (Math|Interpolation|VInterpTo (Transformation|GetWorldLocation (Variables|Default|GetSphere)) (Variables|Default|GetCameraDesiredLocation) (Variables|Default|GetDeltaTime) (Variables|Default|GetCameraInterpSpeed)) false false))

(fn DebugSplineMovement
  (if (Variables|Debug|GetbShowDebug)
    _))

(fn SetDesiredTime
  (bind _outactors (Actor|GetAllActorsOfClass "/Script/Engine.Character"))
  (for _index (range 0 (- (Utilities|Array|Length _outactors) 1))
    (if (!= (Utilities|Array|Get(acopy) _outactors _index) 0)
      (bind _besttime (CallFunction|RecursiveDistanceCheck (Variables|Default|GetSplineIterationMax) 0.001 31.999 (Utilities|Array|Get(acopy) _outactors _index)))
      (if (and (< _besttime (* (Variables|/Script/Engine.SplineComponent|GetDuration (Variables|Default|GetPlayerSpline)) 0.25)) (> (LocalVariables|GetCurrentMax) (* (Variables|/Script/Engine.SplineComponent|GetDuration (Variables|Default|GetPlayerSpline)) 0.75)))
        (LocalVariables|SetCurrentMax _besttime)
        (elif (> _besttime (LocalVariables|GetCurrentMax))
          (LocalVariables|SetCurrentMax _besttime)))))
  (Variables|Default|SetSplineDesiredTime (LocalVariables|GetCurrentMax)))