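; SFPlayercontroller is a player controller that kills its pawn when it leaves the camera's bounds.
; Each tick it asks the CameraFocusActor view target whether the pawn is out of bounds, using a flag to trigger only once.
; ServerHandleGoneOutOfBounds then destroys the pawn and calls ClientsPlayExplosion, which plays a 2D explosion sound.
; Debug strings print at both the detection and sound steps.
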(event `self.ReceiveBeginPlay`)

(event `self.ReceiveTick`
  (params (DeltaSeconds :type "Float (single-precision)"))
  (`parent.ReceiveTick` DeltaSeconds)
  (if (not (or (== (`self.K2_GetPawn`) null) (`self.hasGoneOutOfBounds`)))
    (bind _ascamera_focus_actor (cast `/Game/Blueprints/CameraFocusActor` (`self.GetViewTarget`)))
    (bind _return_value (`/Game/Blueprints/CameraFocusActor.isActorOutOfCameraBounds` _ascamera_focus_actor (`self.K2_GetPawn`)))
    (if _return_value
      (`KismetSystemLibrary.PrintString` null "Out of bounds")
      (set `self.hasGoneOutOfBounds` true)
      (`self.ServerHandleGoneOutOfBounds`))))

(event `ServerHandleGoneOutOfBounds`
  (`self.K2_DestroyActor` (`self.K2_GetPawn`))
  (`self.ClientsPlayExplosion`))

(event `ClientsPlayExplosion`
  (`KismetSystemLibrary.PrintString` null "shouldplay string" true true (struct :`G` 0.66 :`B` 1.0 :`A` 1.0) 10.0)
  (`GameplayStatics.PlaySound2D` null "/Game/StarterContent/Audio/Explosion01.Explosion01"))

(fn `UserConstructionScript`)